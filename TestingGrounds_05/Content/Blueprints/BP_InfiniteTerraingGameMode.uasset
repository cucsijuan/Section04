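; Game mode for an infinite terrain game that spawns a chain of tiles and tracks the number conquered as a score.
; On BeginPlay it populates a nav mesh bounds volume pool, then spawns the initial run of tiles.
; Each new BP_Tile receives the shared pool and supplies the attach point where the next tile spawns.
; NewTileConquered increments the score, and GetScore exposes it.
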(event `self.ReceiveBeginPlay`
  (`self.PopulateBoundsVolumePool`)
  (for _ (range 4)
    (`self.SpawnTile`)))

(fn `GetScore`
  (returns (Score :type Integer))
  (return (`self.Score`)))

(fn `NewTileConquered`
  (`/Engine/EditorBlueprintResources/StandardMacros.IncrementInt` (`self.Score`)))

(fn `SpawnTile`
  (bind _returnvalue (`|SpawnActorFromClass` "/Game/Dynamic/Terrain/BP_Tile.BP_Tile_C" (`self.LastTransformLocation`) "Undefined" "OverrideRootScale" null null))
  (`Tile.SetPool` _returnvalue (`self.NavMeshBoundsVolumePool`))
  (bind _attachtransform (`/Game/Dynamic/Terrain/BP_Tile.GetAttachLocation` _returnvalue))
  (set `self.LastTransformLocation` _attachtransform))

(fn `UserConstructionScript`)